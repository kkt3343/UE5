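; BP_MyGameMode is a game mode Blueprint with an unfinished player respawn system.
; BeginPlay stores the transform of player start "0" and binds RespawnPlayer to the player pawn's destruction.
; Both respawn handlers call RevivePlayer, which is empty.
; The nodes to spawn BP_MyCharacter2, possess it and bind RespawnPlayer2 are disconnected, so no respawn occurs.
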(event `self.ReceiveBeginPlay`
  (set `self.SpawnTransform` (`self.GetTransform` (`self.K2_FindPlayerStart` null "0")))
  (add `self.OnDestroyed` (`GameplayStatics.GetPlayerPawn` 0) (delegate `RespawnPlayer`)))

(event `RespawnPlayer` :!signature `self.OnDestroyed`
  (params (DestroyedActor :type "Actor Object Reference"))
  (`self.RevivePlayer`))

(event `RevivePlayer`)

(event `RespawnPlayer2` :!signature `self.OnDestroyed`
  (params (DestroyedActor :type "Actor Object Reference"))
  (`self.RevivePlayer`))

(fn `UserConstructionScript`)